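; Potion liquid actor: a cylinder with a dynamic material, point light and Niagara bubbles, starting as glowing, bubbly potion.
; TriggerColorChange sets a target that Tick approaches in fixed per-channel steps, updating material, light and bubbles until within tolerance.
; IsWater switches between unlit water, which always bubbles, and lit potion with optional bubbles.
; RotateLiquid never increments its angle, and ChangeBrightness targets a parameter named None.
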(event `self.ReceiveBeginPlay`
  (bind _cylinder (`self.Cylinder`))
  (`self.IsWater` false true)
  (bind _returnvalue (`PrimitiveComponent.CreateDynamicMaterialInstance` _cylinder 0 (`PrimitiveComponent.GetMaterial` _cylinder 0) "None"))
  (bind _returnvalue_2 (`MaterialInstanceDynamic.K2_GetVectorParameterValue` _returnvalue "Inner Color"))
  (bind _output_get (set `self.CurrentColor` (`KismetMathLibrary.Conv_LinearColorToVector` _returnvalue_2)))
  (`LightComponent.SetLightColor` (`self.PointLight`) (`KismetMathLibrary.Conv_VectorToLinearColor` _output_get) true)
  (`NiagaraComponent.SetVariableMaterial` (`self.NS_Bubbles`) "ChangeMaterial" (`PrimitiveComponent.GetMaterial` (`self.Cylinder`) 0)))

(event `self.ReceiveTick`
  (params (DeltaSeconds :type "Float (single-precision)"))
  (`self.CheckForColorChange`))

(event `ChangeColor`
  (params (Color :type "Vector Structure"))
  (bind _currentcolor_x (`KismetMathLibrary.BreakVector` (`self.CurrentColor`)))
  (bind (_currentcolor_x_2 _currentcolor_y _currentcolor_z) (`KismetMathLibrary.BreakVector` (`self.CurrentColor`)))
  (bind (_currentcolor_x_3 _currentcolor_y_2 _currentcolor_z_2) (`KismetMathLibrary.BreakVector` (`self.CurrentColor`)))
  (bind (_currentcolor_x_4 _currentcolor_y_3 _currentcolor_z_3) (`KismetMathLibrary.BreakVector` (`self.CurrentColor`)))
  (bind (_currentcolor_x_5 _currentcolor_y_4 _currentcolor_z_4) (`KismetMathLibrary.BreakVector` (`self.CurrentColor`)))
  (bind (_currentcolor_x_6 _currentcolor_y_5 _currentcolor_z_5) (`KismetMathLibrary.BreakVector` (`self.CurrentColor`)))
  (bind (_currentcolor_x_7 _currentcolor_y_6) (`KismetMathLibrary.BreakVector` (`self.CurrentColor`)))
  (bind (_currentcolor_x_8 _currentcolor_y_7 _currentcolor_z_6) (`KismetMathLibrary.BreakVector` (`self.CurrentColor`)))
  (bind (_currentcolor_x_9 _currentcolor_y_8 _currentcolor_z_7) (`KismetMathLibrary.BreakVector` (`self.CurrentColor`)))
  (set `self.ColorChanged` false)
  (if (< _currentcolor_x Color_X)
    (set `self.CurrentColor` (`KismetMathLibrary.MakeVector` (+ _currentcolor_x_5 0.01) _currentcolor_y_4 _currentcolor_z_4))
    (else
      (set `self.CurrentColor` (`KismetMathLibrary.MakeVector` (- _currentcolor_x_6 0.01) _currentcolor_y_5 _currentcolor_z_5))))
  (if (< _currentcolor_y_6 Color_Y)
    (set `self.CurrentColor` (`KismetMathLibrary.MakeVector` _currentcolor_x_8 (+ _currentcolor_y_7 0.01) _currentcolor_z_6))
    (else
      (set `self.CurrentColor` (`KismetMathLibrary.MakeVector` _currentcolor_x_9 (- _currentcolor_y_8 0.01) _currentcolor_z_7))))
  (if (< _currentcolor_z_3 Color_Z)
    (bind _output_get (set `self.CurrentColor` (`KismetMathLibrary.MakeVector` _currentcolor_x_3 _currentcolor_y_2 (+ _currentcolor_z_2 0.01))))
    (else
      (set `self.CurrentColor` (`KismetMathLibrary.MakeVector` _currentcolor_x_2 _currentcolor_y (- _currentcolor_z 0.01)))))
  (`MeshComponent.SetVectorParameterValueOnMaterials` (`self.Cylinder`) "Inner Color" _output_get)
  (`NiagaraComponent.SetVariableMaterial` (`self.NS_Bubbles`) "ChangeMaterial" (`PrimitiveComponent.GetMaterial` (`self.Cylinder`) 0))
  (`LightComponent.SetLightColor` (`self.PointLight`) (`KismetMathLibrary.Conv_VectorToLinearColor` (`self.CurrentColor`)) true)
  (if (== (`self.CurrentColor`) (`KismetMathLibrary.MakeVector` Color_X Color_Y Color_Z) :`ErrorTolerance` 0.01)
    (set `self.ColorChanged` true)))

(event `CheckForColorChange`
  (if (`self.ChangeColorFlag`)
    (`self.ChangeColor` (`self.NewColor`))
    (if (`self.ColorChanged`)
      (set `self.ChangeColorFlag` false))))

(event `TriggerColorChange`
  (params (NewColor :type "Vector Structure"))
  (set `self.NewColor` NewColor)
  (set `self.ChangeColorFlag` true))

(event `RotateLiquid`
  (if (< (`self.Rotate`) 360.0)
    (`SceneComponent.K2_SetWorldRotation` (`self.DefaultSceneRoot`) (`KismetMathLibrary.MakeRotator` 0.0 0.0 (`self.Rotate`)) false false)
    (else
      (set `self.Rotate` 0.0))))

(event `ChangeBrightness`
  (params (Brightness :type "Float (double-precision)"))
  (`MeshComponent.SetScalarParameterValueOnMaterials` (`self.Cylinder`) "None" Brightness))

(event `BubblesVisible`
  (params (isVisible :type Boolean))
  (if isVisible
    (`SceneComponent.SetVisibility` (`self.NS_Bubbles`) true false)
    (else
      (`SceneComponent.SetVisibility` (`self.NS_Bubbles`) false false))))

(event `IsWater`
  (params (isWater :type Boolean) (isBubbly :type Boolean))
  (if isWater
    (`PrimitiveComponent.SetMaterial` (`self.Cylinder`) 0 "/Game/Materials/M_Water_Inst.M_Water_Inst")
    (`LightComponent.SetIntensity` (`self.PointLight`) 0.0)
    (if true
      (`self.BubblesVisible` true)
      (else
        (`self.BubblesVisible` false)))
    (else
      (`PrimitiveComponent.SetMaterial` (`self.Cylinder`) 0 "/Game/Materials/M_PotionLiquid_Inst.M_PotionLiquid_Inst")
      (`LightComponent.SetIntensity` (`self.PointLight`) 100.0)
      (if isBubbly
        (`self.BubblesVisible` true)
        (else
          (`self.BubblesVisible` false))))))

(fn `UserConstructionScript`)