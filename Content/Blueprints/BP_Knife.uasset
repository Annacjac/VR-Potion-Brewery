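; BP_Knife is a grabbable knife actor that returns to its starting place when dropped.
; It records its root's world transform on BeginPlay and teleports back to it whenever the GrabComponent reports a drop.
; While held, it enables player input and adds an Enhanced Input mapping context, removing both on release, though this graph defines no input actions.
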(event `self.ReceiveBeginPlay`
  (set `self.OriginalPosition` (`SceneComponent.K2_GetComponentToWorld` (`self.DefaultSceneRoot`))))

(event `self.GrabComponent.OnGrabbed`
  (`self.EnableInput` (`GameplayStatics.GetPlayerController` 0))
  (`EnhancedInputSubsystemInterface.AddMappingContext` (pcsubsystem `EnhancedInputLocalPlayerSubsystem` (`GameplayStatics.GetPlayerController` 0)) null 1 (struct)))

(event `self.GrabComponent.OnDropped`
  (`self.DisableInput` (`GameplayStatics.GetPlayerController` 0))
  (`EnhancedInputSubsystemInterface.RemoveMappingContext` (pcsubsystem `EnhancedInputLocalPlayerSubsystem` (`GameplayStatics.GetPlayerController` 0)) null (struct))
  (`self.ResetPosition`))

(event `ResetPosition`
  (`SceneComponent.K2_SetWorldTransform` (`self.DefaultSceneRoot`) (`self.OriginalPosition`) false true))

(fn `UserConstructionScript`)