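; BP_SolidIngredient is a grabbable, physics-simulated solid ingredient that can be crushed or cut.
; InitializeItem copies the ID's row from DT_IngredientDetails, then uses size and ID to add a mesh at runtime, setting quantity and a "Bunch of" or "Bundle of" name.
; CrushItem and CutItem record the preparation and prepend it to the full name.
; Grabbing enables input and adds an Enhanced Input mapping context; dropping reverses both.
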(event `InitializeItem`
  (params (IdNumber :type Integer) (Size :type Integer))
  (bind _name (`self.Name`))
  (bind _returnvalue (`|ForEachDataTableRow` "/Game/Blueprints/DT_IngredientDetails.DT_IngredientDetails")
    (:`Loop Body`
      (if (not (`self.IngredientFound`))
        (bind (_idnumber _name_2 _color _effectsid) (break `/Game/Blueprints/Struct_IngredientDetails` _returnvalue))
        (if (== _idnumber IdNumber)
          (bind _output_get (set `self.IdNumber` _idnumber))
          (set `self.Name` _name_2)
          (set `self.Quantity` Size)
          (set `self.Color` _color)
          (set `self.Effects` _effectsid)
          (switch `int` Size
            (:`1`
              (switch `int` _output_get
                (:`0`
                  (bind _returnvalue_2 (`AddComponent|NODE_AddStaticMeshComponent-0`))
                  (bind _output_get_2 (set `self.Mesh` _returnvalue_2)))
                (:`1`
                  (bind _returnvalue_3 (`AddComponent|NODE_AddStaticMeshComponent-1`))
                  (bind _output_get_3 (set `self.Mesh` _returnvalue_3)))
                (:`2`
                  (bind _returnvalue_4 (`AddComponent|NODE_AddStaticMeshComponent-5`))
                  (bind _output_get_4 (set `self.Mesh` _returnvalue_4)))
                (:`3`
                  (bind _returnvalue_5 (`AddComponent|NODE_AddStaticMeshComponent-6`))
                  (bind _output_get_5 (set `self.Mesh` _returnvalue_5)))
                (:`4`
                  (bind _returnvalue_6 (`AddComponent|NODE_AddStaticMeshComponent-7`))
                  (bind _output_get_6 (set `self.Mesh` _returnvalue_6))))
              (set `self.FullName` (`KismetStringLibrary.Concat_StrStr` "Bunch of " _name))
              (set `self.Quantity` 5))
            (:`2`
              (switch `int` _output_get
                (:`0`
                  (bind _returnvalue_7 (`AddComponent|NODE_AddStaticMeshComponent-8`))
                  (bind _output_get_7 (set `self.Mesh` _returnvalue_7)))
                (:`1`
                  (bind _returnvalue_8 (`AddComponent|NODE_AddStaticMeshComponent-9`))
                  (bind _output_get_8 (set `self.Mesh` _returnvalue_8)))
                (:`2`
                  (bind _returnvalue_9 (`AddComponent|NODE_AddStaticMeshComponent-10`))
                  (bind _output_get_9 (set `self.Mesh` _returnvalue_9)))
                (:`3`
                  (bind _returnvalue_10 (`AddComponent|NODE_AddStaticMeshComponent-11`))
                  (bind _output_get_10 (set `self.Mesh` _returnvalue_10)))
                (:`4`
                  (bind _returnvalue_11 (`AddComponent|NODE_AddStaticMeshComponent-12`))
                  (bind _output_get_11 (set `self.Mesh` _returnvalue_11))))
              (set `self.FullName` (`KismetStringLibrary.Concat_StrStr` "Bundle of " _name))
              (`SceneComponent.K2_AddRelativeRotation` (`self.Mesh`) (struct :`Yaw` -90.0 :`Roll` -90.0) false false)
              (set `self.Quantity` 10)))
          (`PrimitiveComponent.SetSimulatePhysics` _output_get_2 true)
          (`PrimitiveComponent.SetSimulatePhysics` _output_get_3 true)
          (`PrimitiveComponent.SetSimulatePhysics` _output_get_4 true)
          (`PrimitiveComponent.SetSimulatePhysics` _output_get_5 true)
          (`PrimitiveComponent.SetSimulatePhysics` _output_get_6 true)
          (`PrimitiveComponent.SetSimulatePhysics` _output_get_7 true)
          (`PrimitiveComponent.SetSimulatePhysics` _output_get_8 true)
          (`PrimitiveComponent.SetSimulatePhysics` _output_get_9 true)
          (`PrimitiveComponent.SetSimulatePhysics` _output_get_10 true)
          (`PrimitiveComponent.SetSimulatePhysics` _output_get_11 true))))))

(event `self.ReceiveBeginPlay`)

(event `CrushItem`
  (bind _output_get (set `self.Preparation` "Crushed"))
  (set `self.FullName` (`KismetStringLibrary.Concat_StrStr` _output_get " " (`self.FullName`))))

(event `self.GrabComponent.OnGrabbed`
  (`self.EnableInput` (`GameplayStatics.GetPlayerController` 0))
  (`EnhancedInputSubsystemInterface.AddMappingContext` (pcsubsystem `EnhancedInputLocalPlayerSubsystem` (`GameplayStatics.GetPlayerController` 0)) null 1 (struct)))

(event `CutItem`
  (bind _output_get (set `self.Preparation` "Cut"))
  (set `self.FullName` (`KismetStringLibrary.Concat_StrStr` _output_get " " (`self.FullName`))))

(event `self.GrabComponent.OnDropped`
  (`self.DisableInput` (`GameplayStatics.GetPlayerController` 0))
  (`EnhancedInputSubsystemInterface.RemoveMappingContext` (pcsubsystem `EnhancedInputLocalPlayerSubsystem` (`GameplayStatics.GetPlayerController` 0)) null (struct)))

(fn `UserConstructionScript`)