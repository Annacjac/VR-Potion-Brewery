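; Modular interior window Blueprint that fakes a looping day cycle through its rect light and window mesh materials.
; Tick calls DayCycle, whose Delay nodes throttle single-unit intensity steps up or down according to a Sunrise flag, with longer pauses at both extremes.
; A Brightness counter steps alongside the light and feeds a scaled "Brightness" scalar parameter to the window's materials.
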(event `self.ReceiveTick`
  (params (DeltaSeconds :type "Float (single-precision)"))
  (`self.DayCycle`))

(event `DayCycle`
  (if (and (< (`LightComponentBase.Intensity` (`self.RectLight`)) 100.0) (`self.Sunrise`))
    (`KismetSystemLibrary.Delay` 0.2)
    (`LightComponent.SetIntensity` (`self.RectLight`) (+ (`LightComponentBase.Intensity` (`self.RectLight`)) 1.0))
    (bind _result (`/Engine/EditorBlueprintResources/StandardMacros.IncrementFloat` (`self.Brightness`))
      (:`  `
        (`MeshComponent.SetScalarParameterValueOnMaterials` (`self.MOD_Window_interior_03`) "Brightness" (* _result 0.01))))
    (elif (== (`LightComponentBase.Intensity` (`self.RectLight`)) 100.0)
      (set `self.Sunrise` false)
      (`KismetSystemLibrary.Delay` 5.0)
      (`LightComponent.SetIntensity` (`self.RectLight`) (- (`LightComponentBase.Intensity` (`self.RectLight`)) 1.0))
      (bind _result_2 (`/Engine/EditorBlueprintResources/StandardMacros.DecrementFloat` (`self.Brightness`))
        (:`  `
          (`MeshComponent.SetScalarParameterValueOnMaterials` (`self.MOD_Window_interior_03`) "Brightness" (* _result_2 0.01))))
      (elif (> (`LightComponentBase.Intensity` (`self.RectLight`)) 0.0)
        (`KismetSystemLibrary.Delay` 0.2)
        (`LightComponent.SetIntensity` (`self.RectLight`) (- (`LightComponentBase.Intensity` (`self.RectLight`)) 1.0))
        (bind _result_3 (`/Engine/EditorBlueprintResources/StandardMacros.DecrementFloat` (`self.Brightness`))
          (:`  `
            (`MeshComponent.SetScalarParameterValueOnMaterials` (`self.MOD_Window_interior_03`) "Brightness" (* _result_3 0.01))
            (if (== (`LightComponentBase.Intensity` (`self.RectLight`)) 0.0)
              (`KismetSystemLibrary.Delay` 5.0)
              (set `self.Sunrise` true))))))))

(fn `UserConstructionScript`)