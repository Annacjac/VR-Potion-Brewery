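; Modular interior window that fakes a day/night cycle with a RectLight and the emissive material on its window mesh.
; BeginPlay uses the Day flag to set a bright warm or dim blue starting state.
; Tick calls DayCycle, where Delay nodes pace single steps of light intensity and material Brightness.
; The Sunrise flag sets direction, colors switch at intensity thresholds, and long delays hold full day and night.
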(event `self.ReceiveBeginPlay`
  (if (`self.Day`)
    (`MeshComponent.SetScalarParameterValueOnMaterials` (`self.MOD_Window_interior_03`) "Brightness" 1.0)
    (`LightComponent.SetLightColor` (`self.RectLight`) (struct :`R` 1.0 :`G` 0.807843 :`B` 0.439216 :`A` 1.0) true)
    (`MeshComponent.SetVectorParameterValueOnMaterials` (`self.MOD_Window_interior_03`) "Emission Color" (1.0 0.23208 0.0))
    (`LightComponent.SetIntensity` (`self.RectLight`) 130.0)
    (set `self.Brightness` 101.0)
    (else
      (`MeshComponent.SetScalarParameterValueOnMaterials` (`self.MOD_Window_interior_03`) "Brightness" 0.01)
      (`LightComponent.SetLightColor` (`self.RectLight`) (struct :`R` 0.156863 :`G` 0.184314 :`B` 0.376471 :`A` 1.0) true)
      (`MeshComponent.SetVectorParameterValueOnMaterials` (`self.MOD_Window_interior_03`) "Emission Color" (0.110107 0.289884 0.640625))
      (`LightComponent.SetIntensity` (`self.RectLight`) 30.0)
      (set `self.Brightness` 1.0))))

(event `self.ReceiveTick`
  (params (DeltaSeconds :type "Float (single-precision)"))
  (`self.DayCycle`))

(event `DayCycle`
  (if (and (< (`LightComponentBase.Intensity` (`self.RectLight`)) 130.0) (`self.Sunrise`))
    (`KismetSystemLibrary.Delay` 1.5)
    (`LightComponent.SetIntensity` (`self.RectLight`) (+ (`LightComponentBase.Intensity` (`self.RectLight`)) 1.0))
    (bind _result (`/Engine/EditorBlueprintResources/StandardMacros.IncrementFloat` (`self.Brightness`))
      (:`  `
        (`MeshComponent.SetScalarParameterValueOnMaterials` (`self.MOD_Window_interior_03`) "Brightness" (* _result 0.01))
        (if (== (`LightComponentBase.Intensity` (`self.RectLight`)) 35.0)
          (`LightComponent.SetLightColor` (`self.RectLight`) (struct :`R` 1.0 :`G` 0.471354 :`B` 0.123204 :`A` 1.0) true)
          (`MeshComponent.SetVectorParameterValueOnMaterials` (`self.MOD_Window_interior_03`) "Emission Color" (1.0 0.317658 0.0))
          (elif (== (`LightComponentBase.Intensity` (`self.RectLight`)) 50.0)
            (`LightComponent.SetLightColor` (`self.RectLight`) (struct :`R` 1.0 :`G` 0.807843 :`B` 0.439216 :`A` 1.0) true)
            (`MeshComponent.SetVectorParameterValueOnMaterials` (`self.MOD_Window_interior_03`) "Emission Color" (1.0 0.23208 0.0))))))
    (elif (== (`LightComponentBase.Intensity` (`self.RectLight`)) 130.0)
      (set `self.Sunrise` false)
      (`KismetSystemLibrary.Delay` 330.0)
      (`LightComponent.SetIntensity` (`self.RectLight`) (- (`LightComponentBase.Intensity` (`self.RectLight`)) 1.0))
      (bind _result_2 (`/Engine/EditorBlueprintResources/StandardMacros.DecrementFloat` (`self.Brightness`))
        (:`  `
          (`MeshComponent.SetScalarParameterValueOnMaterials` (`self.MOD_Window_interior_03`) "Brightness" (* _result_2 0.01))))
      (elif (> (`LightComponentBase.Intensity` (`self.RectLight`)) 30.0)
        (`KismetSystemLibrary.Delay` 1.5)
        (`LightComponent.SetIntensity` (`self.RectLight`) (- (`LightComponentBase.Intensity` (`self.RectLight`)) 1.0))
        (bind _result_3 (`/Engine/EditorBlueprintResources/StandardMacros.DecrementFloat` (`self.Brightness`))
          (:`  `
            (`MeshComponent.SetScalarParameterValueOnMaterials` (`self.MOD_Window_interior_03`) "Brightness" (* _result_3 0.01))
            (if (== (`LightComponentBase.Intensity` (`self.RectLight`)) 50.0)
              (`LightComponent.SetLightColor` (`self.RectLight`) (struct :`R` 1.0 :`G` 0.471354 :`B` 0.123204 :`A` 1.0) true)
              (`MeshComponent.SetVectorParameterValueOnMaterials` (`self.MOD_Window_interior_03`) "Emission Color" (1.0 0.317658 0.0))
              (elif (== (`LightComponentBase.Intensity` (`self.RectLight`)) 35.0)
                (`LightComponent.SetLightColor` (`self.RectLight`) (struct :`R` 0.356863 :`G` 0.423529 :`B` 0.862745 :`A` 1.0) true)
                (`MeshComponent.SetVectorParameterValueOnMaterials` (`self.MOD_Window_interior_03`) "Emission Color" (0.110107 0.289884 0.640625))
                (elif (== (`LightComponentBase.Intensity` (`self.RectLight`)) 30.0)
                  (`KismetSystemLibrary.Delay` 330.0)
                  (set `self.Sunrise` true))))))))))

(fn `UserConstructionScript`)