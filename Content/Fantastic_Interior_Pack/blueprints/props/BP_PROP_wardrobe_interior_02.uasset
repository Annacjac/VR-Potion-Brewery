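; Interactive wardrobe prop whose two doors swing open or shut according to the IsOpen flag, which nothing in these graphs sets.
; Tick calls OpenWardrobe or CloseWardrobe every frame, each stepping the mirrored door yaws by a fixed amount until a limit is reached.
; The motion uses relative rotation without delta time or a timeline, so its speed depends on frame rate.
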(event `self.ReceiveTick`
  (params (DeltaSeconds :type "Float (single-precision)"))
  (if (`self.isOpen`)
    (`self.OpenWardrobe`)
    (else
      (`self.CloseWardrobe`))))

(event `OpenWardrobe`
  (if (and (< (`self.rotationR`) 120.0) (> (`self.rotationL`) -120.0))
    (`SceneComponent.K2_SetRelativeRotation` (`self.SM_PROP_wardrobe_door_01_interior_02`) (`KismetMathLibrary.MakeRotator` 0.0 0.0 (`self.rotationR`)) false false)
    (`SceneComponent.K2_SetRelativeRotation` (`self.SM_PROP_wardrobe_door_02_interior_02`) (`KismetMathLibrary.MakeRotator` 0.0 0.0 (`self.rotationL`)) false false)
    (set `self.rotationR` (+ (`self.rotationR`) 3.0))
    (set `self.rotationL` (- (`self.rotationL`) 3.0))))

(event `CloseWardrobe`
  (if (and (> (`self.rotationR`) 0.0) (< (`self.rotationL`) 0.0))
    (`SceneComponent.K2_SetRelativeRotation` (`self.SM_PROP_wardrobe_door_01_interior_02`) (`KismetMathLibrary.MakeRotator` 0.0 0.0 (`self.rotationR`)) false false)
    (`SceneComponent.K2_SetRelativeRotation` (`self.SM_PROP_wardrobe_door_02_interior_02`) (`KismetMathLibrary.MakeRotator` 0.0 0.0 (`self.rotationL`)) false false)
    (set `self.rotationR` (- (`self.rotationR`) 3.0))
    (set `self.rotationL` (+ (`self.rotationL`) 3.0))))

(fn `UserConstructionScript`)