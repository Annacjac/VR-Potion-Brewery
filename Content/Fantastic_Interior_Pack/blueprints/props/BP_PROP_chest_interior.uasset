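; Interior chest prop whose lid swings open or closed according to the IsOpen flag.
; Every Tick calls OpenChest or CloseChest, which step the lid mesh's relative roll by a fixed amount between closed and a quarter turn open.
; The motion uses no timeline or delta time, so its speed depends on frame rate.
; Nothing in these graphs sets IsOpen.
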(event `self.ReceiveBeginPlay`)

(event `self.ReceiveTick`
  (params (DeltaSeconds :type "Float (single-precision)"))
  (if (`self.isOpen`)
    (`self.OpenChest`)
    (else
      (`self.CloseChest`))))

(event `OpenChest`
  (bind _lidrotation (`self.lidRotation`))
  (if (> (`self.lidRotation`) -90.0)
    (`SceneComponent.K2_SetRelativeRotation` (`self.SM_PROP_chest_lid_interior`) (`KismetMathLibrary.MakeRotator` _lidrotation) false false)
    (set `self.lidRotation` (- _lidrotation 2.0))))

(event `CloseChest`
  (bind _lidrotation (`self.lidRotation`))
  (if (< (`self.lidRotation`) 0.0)
    (`SceneComponent.K2_SetRelativeRotation` (`self.SM_PROP_chest_lid_interior`) (`KismetMathLibrary.MakeRotator` _lidrotation) false false)
    (set `self.lidRotation` (+ _lidrotation 2.0))))

(fn `UserConstructionScript`)